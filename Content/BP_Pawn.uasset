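; Player pawn that runs a Tetris game: spawns random tetromino actors, moves and turns them on input, and clears full rows.
; A map of cell index to cube models the ten-wide board for movement and rotation checks.
; Looping timers drive the fall and held-key movement.
; A blocked fall registers the piece's cubes, spawns the next, then hides full rows, shifts higher cubes down and destroys emptied piece actors.
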(event `self.ReceiveBeginPlay`
  ;[1 1 1] Init GameStatus
  (for _index (range 230)
    (`BlueprintMapLibrary.Map_Add` (`self.Cubes`) _index))
  (`self.SpawnTetris`)
  (`KismetSystemLibrary.K2_SetTimerDelegate` (delegate `DownLoop`) (/ 1.0 (`self.DownLoopSpeed`)) true))

(event `DownLoop`
  (bind _res (`self.CanMoveDown`))
  (if _res
    (`/Game/TetrisCube/BP_Tetris.Move` (`self.TetrisActor`) (0.0 0.0 -100.0))
    (else
      (`KismetSystemLibrary.Delay` (`self.InputDelay`))
      (`self.FinishOneCube`))))

(event `InputAction|Turn`
  (params (Key :type "Key Structure"))
  (:`Pressed`
    (bind _res (`self.CanTurn`))
    (if _res
      (`/Game/TetrisCube/BP_Tetris.Turn` (`self.TetrisActor`)))))

(event `InputAction|MoveRight`
  (params (Key :type "Key Structure"))
  (:`Pressed`
    (`self.MoveRight`)
    (bind _returnvalue (`KismetSystemLibrary.K2_SetTimerDelegate` (delegate `MoveRightLoop`) (/ 1.0 (`self.MoveLeftOrRightSpeed`)) true))
    (set `self.MoveRightTimerHandle` _returnvalue))
  (:`Released`
    (`KismetSystemLibrary.K2_ClearAndInvalidateTimerHandle` (`self.MoveRightTimerHandle`))))

(event `InputAction|MoveLeft`
  (params (Key :type "Key Structure"))
  (:`Pressed`
    (`self.MoveLeft`)
    (bind _returnvalue (`KismetSystemLibrary.K2_SetTimerDelegate` (delegate `MoveLeftLoop`) (/ 1.0 (`self.MoveLeftOrRightSpeed`)) true))
    (set `self.MoveLeftTimerHandle` _returnvalue))
  (:`Released`
    (`KismetSystemLibrary.K2_ClearAndInvalidateTimerHandle` (`self.MoveLeftTimerHandle`))))

(event `MoveRightLoop`
  (`self.MoveRight`))

(event `MoveLeftLoop`
  (`self.MoveLeft`))

(event `InputAction|MoveDown`
  (params (Key :type "Key Structure"))
  (:`Pressed`
    (`self.MoveDown`)
    (bind _returnvalue (`KismetSystemLibrary.K2_SetTimerDelegate` (delegate `MoveDownLoop`) (/ 1.0 (`self.MoveDownSpeed`)) true))
    (set `self.MoveDownTimerHandle` _returnvalue))
  (:`Released`
    (`KismetSystemLibrary.K2_ClearAndInvalidateTimerHandle` (`self.MoveDownTimerHandle`))))

(event `MoveDownLoop`
  (`self.MoveDown`))

(fn `CanMoveDown`
  (returns (Res :type Boolean))
  (bind _tetrisactor (`self.TetrisActor`))
  (bind _statuindexs (`/Game/TetrisCube/BP_Tetris.GetStatuIndexs` _tetrisactor (`/Game/TetrisCube/BP_Tetris.CurrentIndex` _tetrisactor)))
  (for _array_element _statuindexs
    ;[1 1 1] Down edge
    (if (< _array_element 10)
      (return false)
      (else
        ;[1 1 1] Is right empty
        (if (`KismetSystemLibrary.IsValid` (`BlueprintMapLibrary.Map_Find` (`self.Cubes`) (+ _array_element -10)))
          (return false)))))
  (return true))

(fn `CanMoveLeft`
  (returns (Res :type Boolean))
  (bind _tetrisactor (`self.TetrisActor`))
  (bind _statuindexs (`/Game/TetrisCube/BP_Tetris.GetStatuIndexs` _tetrisactor (`/Game/TetrisCube/BP_Tetris.CurrentIndex` _tetrisactor)))
  (for _array_element _statuindexs
    ;[1 1 1] Left edge
    (if (== (mod _array_element 10) 0)
      (return false)
      (else
        ;[1 1 1] Is left empty
        (if (`KismetSystemLibrary.IsValid` (`BlueprintMapLibrary.Map_Find` (`self.Cubes`) (+ _array_element -1)))
          (return false)))))
  (return true))

(fn `CanMoveRight`
  (returns (Res :type Boolean))
  (bind _tetrisactor (`self.TetrisActor`))
  (bind _statuindexs (`/Game/TetrisCube/BP_Tetris.GetStatuIndexs` _tetrisactor (`/Game/TetrisCube/BP_Tetris.CurrentIndex` _tetrisactor)))
  (for _array_element _statuindexs
    (bind _returnvalue (+ _array_element 1))
    ;[1 1 1] Right edge
    (if (== (mod _returnvalue 10) 0)
      (return false)
      (else
        ;[1 1 1] Is right empty
        (if (`KismetSystemLibrary.IsValid` (`BlueprintMapLibrary.Map_Find` (`self.Cubes`) _returnvalue))
          (return false)))))
  (return true))

(fn `CanTurn`
  (returns (Res :type Boolean))
  (bind _tetrisactor (`self.TetrisActor`))
  (bind _returnvalue (`self.K2_GetActorLocation` (`self.TetrisActor`)))
  (bind _outcurrentindex (`/Game/TetrisCube/BP_Tetris.GetNextTetrisIndex` _tetrisactor))
  (bind (_cubeindex1 _cubeindex2 _cubeindex3 _cubeindex4) (break `/Game/TetrisCube/Struct_Tetris` (`|GetArrayItem` (`/Game/TetrisCube/BP_Tetris.Tetris` (`self.TetrisActor`)) _outcurrentindex)))
  (if (or (`self.IsOutPlayGround` (+ _cubeindex1 _returnvalue)) (`self.IsOutPlayGround` (+ _cubeindex2 _returnvalue)) (`self.IsOutPlayGround` (+ _cubeindex3 _returnvalue)) (`self.IsOutPlayGround` (+ _cubeindex4 _returnvalue)))
    (return false)
    (else
      (bind _statuindexs (`/Game/TetrisCube/BP_Tetris.GetStatuIndexs` _tetrisactor _outcurrentindex))
      (for _array_element _statuindexs
        (if (`KismetSystemLibrary.IsValid` (`BlueprintMapLibrary.Map_Find` (`self.Cubes`) _array_element))
          (return false)))
      (return true))))

(fn `FinishOneCube`
  (bind _tetrisactor (`self.TetrisActor`))
  (`|ExecutionSequence`
    (:`then_0`
      ;[1 1 1] Clear MoveLoop TimerHandles
      (`KismetSystemLibrary.K2_ClearAndInvalidateTimerHandle` (`self.MoveLeftTimerHandle`))
      (`KismetSystemLibrary.K2_ClearAndInvalidateTimerHandle` (`self.MoveRightTimerHandle`))
      (`KismetSystemLibrary.K2_ClearAndInvalidateTimerHandle` (`self.MoveDownTimerHandle`))
      (bind _statuindexs (`/Game/TetrisCube/BP_Tetris.GetStatuIndexs` _tetrisactor (`/Game/TetrisCube/BP_Tetris.CurrentIndex` _tetrisactor)))
      (`|ExecutionSequence`
        (:`then_0`
          (`BlueprintMapLibrary.Map_Add` (`self.Cubes`) (`|GetArrayItem` _statuindexs) (`/Game/TetrisCube/BP_Tetris.Cube` (`self.TetrisActor`))))
        (:`then_1`
          (`BlueprintMapLibrary.Map_Add` (`self.Cubes`) (`|GetArrayItem` _statuindexs 1) (`/Game/TetrisCube/BP_Tetris.Cube1` (`self.TetrisActor`))))
        (:`then_2`
          (`BlueprintMapLibrary.Map_Add` (`self.Cubes`) (`|GetArrayItem` _statuindexs 2) (`/Game/TetrisCube/BP_Tetris.Cube2` (`self.TetrisActor`))))
        (:`then_3`
          (`BlueprintMapLibrary.Map_Add` (`self.Cubes`) (`|GetArrayItem` _statuindexs 3) (`/Game/TetrisCube/BP_Tetris.Cube3` (`self.TetrisActor`))))
        (:`then_4`
          (`self.SpawnTetris`))))
    (:`then_1`
      (`self.FInishRow`))))

(fn `FInishRow`
  (locals (RowCubeCount :type Integer) (FinishRowIndexs :type "Array of Integer") (DownRowCount :type Integer))
  (bind _cubes (`self.Cubes`))
  (bind _cubes_2 (`self.Cubes`))
  (`|ExecutionSequence`
    (:`then_0`
      (for _index (range 20)
        (set `local.RowCubeCount` 0)
        (for _index_2 (range 10)
          ;[1 1 1] Cube exist
          (`/Engine/EditorBlueprintResources/StandardMacros.IsValid` (`BlueprintMapLibrary.Map_Find` (`self.Cubes`) (+ _index_2 (* _index 10)))
            (:`Is Valid`
              (`/Engine/EditorBlueprintResources/StandardMacros.IncrementInt` (`local.RowCubeCount`)))
            (:`Is Not Valid`
              (break))))
        (if (== (`local.RowCubeCount`) 10)
          (`KismetArrayLibrary.Array_Add` (`local.FinishRowIndexs`) _index))))
    (:`then_1`
      (for _index_3 (range 20)
        (if (`KismetArrayLibrary.Array_Contains` (`local.FinishRowIndexs`) _index_3)
          (for _index_4 (range 10)
            (bind _returnvalue (* _index_3 10))
            (bind _returnvalue_2 (+ _index_4 _returnvalue))
            (`SceneComponent.SetVisibility` (`BlueprintMapLibrary.Map_Find` _cubes _returnvalue_2) false false)
            (`BlueprintMapLibrary.Map_Add` _cubes _returnvalue_2))
          (`/Engine/EditorBlueprintResources/StandardMacros.IncrementInt` (`local.DownRowCount`))
          (elif (> (`local.DownRowCount`) 0)
            (for _index_5 (range 10)
              (bind _returnvalue_3 (+ _returnvalue _index_5))
              (bind _value (`BlueprintMapLibrary.Map_Find` (`self.Cubes`) _returnvalue_3))
              (`/Engine/EditorBlueprintResources/StandardMacros.IsValid` _value
                (:`Is Valid`
                  (`SceneComponent.K2_AddWorldOffset` _value (* (0.0 0.0 -100.0) (`local.DownRowCount`)) false false)
                  (`BlueprintMapLibrary.Map_Add` _cubes_2 (- _returnvalue_3 (* (`local.DownRowCount`) 10)) _value)
                  (`BlueprintMapLibrary.Map_Add` _cubes_2 _returnvalue_3))))))))
    (:`then_2`
      ;[1 1 1] 摧毁被完全消除的Actor
      (bind _outactors (`GameplayStatics.GetAllActorsOfClass` "/Game/TetrisCube/BP_Tetris.BP_Tetris_C"))
      (for _array_element _outactors
        (bind _res (`/Game/TetrisCube/BP_Tetris.IsAllCubesDisable` _array_element))
        (if _res
          (`self.K2_DestroyActor` _array_element))))))

(fn `MoveDown`
  (bind _res (`self.CanMoveDown`))
  (if _res
    (`/Game/TetrisCube/BP_Tetris.Move` (`self.TetrisActor`) (0.0 0.0 -100.0))))

(fn `MoveLeft`
  (bind _res (`self.CanMoveLeft`))
  (if _res
    (`/Game/TetrisCube/BP_Tetris.Move` (`self.TetrisActor`) (0.0 -100.0 0.0))))

(fn `MoveRight`
  (bind _res (`self.CanMoveRight`))
  (if _res
    (`/Game/TetrisCube/BP_Tetris.Move` (`self.TetrisActor`) (0.0 100.0 0.0))))

(fn `SpawnTetris`
  (bind _returnvalue (`|SpawnActorFromClass` (`|GetArrayItem` (`self.TetrisClasses`) (`KismetMathLibrary.RandomIntegerInRange` 0 (- (`KismetArrayLibrary.Array_Length` (`self.TetrisClasses`)) 1))) (`KismetMathLibrary.MakeTransform` (0.0 300.0 1900.0)) "Undefined" "OverrideRootScale" null null))
  (set `self.TetrisActor` _returnvalue))

(fn `UserConstructionScript`)