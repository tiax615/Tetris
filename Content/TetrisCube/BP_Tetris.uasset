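; Tetris piece actor built from four cubes, with rotation states stored as cube offsets in the Tetris array.
; SetCube, run at construction, places the cubes for the current state and tints each through a dynamic material instance.
; Turn cycles the state and re-applies it, while Move offsets the whole actor locally.
; GetStatuIndexs collects per-cube indices, though GetStatuIndex's world Y/Z formula is left unconnected.
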(event `self.ReceiveBeginPlay`)

(fn `GetStatuIndexs`
  (returns (StatuIndexs :type "Array of Integer"))
  (return (`|MakeArray` (`self.GetStatuIndex` (`self.Cube`)) (`self.GetStatuIndex` (`self.Cube1`)) (`self.GetStatuIndex` (`self.Cube2`)) (`self.GetStatuIndex` (`self.Cube3`)))))

(fn `Move`
  (params (InOffset :type "Vector Structure"))
  (`self.K2_AddActorLocalOffset` InOffset))

(fn `SetCube`
  (bind (_cubeindex1 _cubeindex2 _cubeindex3 _cubeindex4) (break `/Game/TetrisCube/Struct_Tetris` (`|GetArrayItem` (`self.Tetris`) (`self.CurrentIndex`))))
  (if (`KismetArrayLibrary.Array_IsValidIndex` (`self.Tetris`))
    (`|ExecutionSequence`
      (:`then_0`
        (`self.SetCubeLocationAndColor` (`self.Cube`) _cubeindex1))
      (:`then_1`
        (`self.SetCubeLocationAndColor` (`self.Cube1`) _cubeindex2))
      (:`then_2`
        (`self.SetCubeLocationAndColor` (`self.Cube2`) _cubeindex3))
      (:`then_3`
        (`self.SetCubeLocationAndColor` (`self.Cube3`) _cubeindex4)))))

(fn `SetCubeLocationAndColor`
  (params (InCube :type "StaticMeshComponent Object Reference") (InRelativeLocation :type "Vector Structure"))
  (bind _returnvalue (`PrimitiveComponent.CreateDynamicMaterialInstance` InCube 0 "/Game/MI_Cube.MI_Cube" "None"))
  (`MaterialInstanceDynamic.SetVectorParameterValue` _returnvalue "Color" (`self.Color`))
  (`SceneComponent.K2_SetRelativeLocation` InCube InRelativeLocation false false))

(fn `Turn`
  (bind _result (`/Engine/EditorBlueprintResources/StandardMacros.IncrementInt` (`self.CurrentIndex`))
    (:`  `
      (if (>= _result (`KismetArrayLibrary.Array_Length` (`self.Tetris`)))
        (set `self.CurrentIndex` 0))
      (`self.SetCube`))))

(fn `UserConstructionScript`
  (`self.SetCube`))